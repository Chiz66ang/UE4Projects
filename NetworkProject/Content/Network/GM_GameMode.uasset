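; GM_GameMode is a last-man-standing game mode that tracks players and assigns spawn points.
; PostLogin adds each controller to PClist, and Remove_PC takes one out.
; When one controller remains after a removal, it calls PlayerWin on that player's ThirdPersonCharacter.
; ChoosePlayerStart picks the first PlayerStart not tagged "Taken" and tags it, falling back to the last one when all are taken.
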(event Custom|Remove_PC
  (params (PC :type Player%20Controller%20Object%20Reference))
  (bind _pclist (Variables|Default|GetPClist))
  ;[1 1 1] Bring all PC that logged in/ Remove PC that are dead/ Show Player Win to last man standing
  (Utilities|Array|RemoveItem _pclist PC)
  (Development|PrintString "removed")
  (if (== (Utilities|Array|Length _pclist) 1)
    (bind _asthird_person_character (Utilities|Casting|CastToThirdPersonCharacter (Pawn|GetControlledPawn (Utilities|Array|Get(acopy) (Variables|Default|GetPClist)))))
    (Default|PlayerWin _asthird_person_character)))

(event EventBeginPlay)

(event EventTick
  (params (DeltaSeconds :type Float%20%28single-precision%29)))

(event EventPostLogin
  (params (NewPlayer :type Player%20Controller%20Object%20Reference))
  ;[1 1 1] Bring all PC that logged in/ Remove PC that are dead/ Show Player Win to last man standing
  (Utilities|Array|Add (Variables|Default|GetPClist) NewPlayer))

(fn ConstructionScript)

(fn ChoosePlayerStart
  (params (Player :type Controller%20Object%20Reference))
  (bind _outactors (Actor|GetAllActorsOfClass "/Script/Engine.PlayerStart"))
  (bind _array_element (Utilities|Array|ForEachLoopwithBreak _outactors :!label _label) ; 아직 점유되지 않은 PlayerStart 검사/ 점유되지 않았으면 Break
    (:LoopBody
      (if (Utilities|Name|NotEqual(Name) (Variables|/Script/Engine.PlayerStart|GetPlayerStartTag _array_element) "Taken")
        (Variables|/Script/Engine.PlayerStart|SetPlayerStartTag _array_element "Taken")
        (goto _label Break)))
    (:Completed
      (Transformation|SetActorScale3D _array_element "1.000000,1.000000,1.000000")
      (return _array_element))))