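; Lobby player controller that shows host and client lobby screens and reveals the game start button to the host.
; On BeginPlay, the local controller creates the lobby widget, shows the cursor and displays a server or client message based on authority.
; Remote clients then call the ServerImHere RPC, which makes the server clear all widgets and add the start button widget.
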(event Custom|ServerImHere!
  (Development|PrintString "Hello!")
  (Networking|SwitchHasAuthority
    (:Authority
      (Viewport|RemoveAllWidgets)
      (bind _returnvalue (UserInterface|CreateWidget "/Game/Network/Lobby/WG_GameStartButton.WG_GameStartButton_C"))
      (UserInterface|Viewport|AddtoViewport _returnvalue 0))))

(event EventBeginPlay
  (if (Pawn|IsLocalPlayerController)
    (bind _returnvalue (UserInterface|CreateWidget "/Game/Network/Lobby/WG_Lobby.WG_Lobby_C" self))
    (UserInterface|Viewport|AddtoViewport _returnvalue 0)
    (Variables|Default|SetbShowMouseCursor true)
    (Networking|SwitchHasAuthority
      (:Authority
        (Widget|SetVisibility (Variables|/Game/Network/Lobby/WG_Lobby.WG_Lobby_C|GetServerMessage _returnvalue) "Visible"))
      (:Remote
        (Widget|SetVisibility (Variables|/Game/Network/Lobby/WG_Lobby.WG_Lobby_C|GetClient_Message _returnvalue) "Visible")
        (CallFunction|ServerImHere!)))))

(event EventTick
  (params (DeltaSeconds :type Float%20%28single-precision%29)))

(fn ConstructionScript)