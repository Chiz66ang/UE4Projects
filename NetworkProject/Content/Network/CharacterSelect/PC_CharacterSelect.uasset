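; Player controller for character selection that shows the selection widget and previews the chosen character as a possessed pawn.
; On BeginPlay, the local controller loads the player save and continues only if its PlayerID is found in the game instance.
; It then opens the widget in UI-only input and spawns the first class from ArrClassRef.
; CreateCharacter destroys the first Character found, then spawns and possesses the class at the given index.
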(event Custom|CreateCharacter
  (params (Character%20Index :type Integer))
  ;[1 1 1] Called when pressed widget button/ Spawn different Characters
  (bind _outactors (Actor|GetAllActorsOfClass "/Script/Engine.Character"))
  (Actor|DestroyActor (Utilities|Array|Get(acopy) _outactors))
  (bind _returnvalue (Game|SpawnActorfromClass (Utilities|Array|Get(acopy) (Variables|Default|GetArrClassRef) Character%20Index) (Math|Transform|MakeTransform "0, 0, 0") "Undefined" 0 0))
  (Transformation|SetRelativeRotation (Variables|/Script/Engine.Character|GetMesh _returnvalue) "0,90.000000, 0" false false)
  (Pawn|UnPossess)
  (Pawn|Possess _returnvalue))

(event Custom|Create%20widget
  ;[1 1 1] Create Character Select Widget/ Spawn first actor
  (bind _returnvalue (UserInterface|CreateWidget "/Game/Network/CharacterSelect/WG_CharacterSelect.WG_CharacterSelect_C" self))
  (bind _output_get (Variables|Default|SetSelectionWG _returnvalue))
  (UserInterface|Viewport|AddtoViewport _output_get 0)
  (Input|SetInputModeUIOnly self 0 "DoNotLock")
  (Variables|Default|SetbShowMouseCursor true)
  (bind _returnvalue_2 (Game|SpawnActorfromClass (Utilities|Array|Get(acopy) (Variables|Default|GetArrClassRef)) (Math|Transform|MakeTransform "0, 0, 0") "Undefined" 0 0))
  (Transformation|SetRelativeRotation (Variables|/Script/Engine.Character|GetMesh _returnvalue_2) "0,90.000000, 0" false false)
  (Pawn|Possess _returnvalue_2))

(event EventBeginPlay
  ;[1 1 1] Check if it is the logged in player
  (if (Pawn|IsLocalPlayerController self)
    (bind _returnvalue (SaveGame|LoadGamefromSlot (Variables|/Game/Network/GI_GameInstance.GI_GameInstance_C|GetSG_SlotName (.AsGI%20Game%20Instance (Utilities|Casting|CastToGI_GameInstance (Game|GetGameInstance))))))
    (bind _assg_player (Utilities|Casting|CastToSG_Player _returnvalue))
    (if (Utilities|Enum|NotEqual(Enum) (Variables|/Game/Network/SG_Player.SG_Player_C|GetPlayerID _assg_player) "")
      (bind _asgi_game_instance (Utilities|Casting|CastToGI_GameInstance (Game|GetGameInstance)))
      (if (.ReturnValue (Utilities|Map|Find (Variables|/Game/Network/GI_GameInstance.GI_GameInstance_C|GetPlayerID _asgi_game_instance) (Variables|/Game/Network/SG_Player.SG_Player_C|GetPlayerID _assg_player)))
        (Variables|Default|SetPC_ID (Variables|/Game/Network/SG_Player.SG_Player_C|GetPlayerID _assg_player))
        (CallFunction|CreateWidget)))))

(fn ConstructionScript)