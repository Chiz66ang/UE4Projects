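; Cube actor that glows, then turns red and explodes once something overlaps its Box component.
; A dynamic material instance created at BeginPlay receives Tick updates to Emissive, using ValueChange to pick the step's sign at the lower and upper limits.
; An overlap sets IsExplode, which zeroes the glow and blends white to red in HSV.
; When the blend completes, Explotion waits briefly, spawns an explosion emitter and destroys the actor.
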(event OnComponentBeginOverlap(Box)
  (params (OverlappedComponent :type Primitive%20Component%20Object%20Reference) (OtherActor :type Actor%20Object%20Reference) (OtherComp :type Primitive%20Component%20Object%20Reference) (OtherBodyIndex :type Integer) (bFromSweep :type Boolean) (SweepResult :type Hit%20Result%20Structure%20%28by%20ref%29))
  (Variables|Default|SetIsExplode true))

(event Custom|Explotion
  ;[1 1 1] Explosion Event
  (Utilities|FlowControl|Delay 0.5)
  (bind _returnvalue (Effects|SpawnEmitteratLocation "/Game/StarterContent/Particles/P_Explosion.P_Explosion" (Transformation|GetActorLocation)))
  (Utilities|FlowControl|Delay 0.0)
  (Components|Activation|Deactivate _returnvalue)
  (Actor|DestroyActor))

(event EventBeginPlay
  (bind _returnvalue (Rendering|Material|CreateDynamicMaterialInstance (Variables|Default|GetCube) 0 0 "None" :!class /Script/Engine.PrimitiveComponent))
  (bind _output_get (Variables|Default|SetDyna%20Mat _returnvalue))
  (Rendering|Material|SetVectorParameterValue _output_get "Custom Color" "(R=1.000000,G=1.000000,B=1.000000,A=1.000000)" :!class /Script/Engine.MaterialInstanceDynamic))

(event Collision|EventActorBeginOverlap
  (params (OtherActor :type Actor%20Object%20Reference)))

(event EventTick
  (params (DeltaSeconds :type Float%20%28single-precision%29))
  (if (Variables|Default|GetIsExplode)
    (bind _output_get (Variables|Default|SetEmissive 0.0)) ; Set Emissive 0
    (Rendering|Material|SetScalarParameterValue (Variables|Default|GetDyna%20Mat) "Emissive" _output_get :!class /Script/Engine.MaterialInstanceDynamic)
    ;[1 1 1] Color Change
    (bind _output_get_2 (Variables|Default|SetAlpha (+ (* DeltaSeconds 0.5) (Variables|Default|GetAlpha))))
    (Rendering|Material|SetVectorParameterValue (Variables|Default|GetDyna%20Mat) "Custom Color" (Class|KismetMathLibrary|LinearColorLerpUsingHSV "(R=1.000000,G=1.000000,B=1.000000,A=1.000000)" "(R=1.000000,G=0.000000,B=0.000000,A=1.000000)" _output_get_2) :!class /Script/Engine.MaterialInstanceDynamic)
    (if (>= (Variables|Default|GetAlpha) 1.0)
      (CallFunction|Explotion))
    (else
      ;[1 1 1] Emission
      (bind _changed_ds (CallFunction|ValueChange DeltaSeconds)) ; 발광 함수
      (bind _output_get_3 (Variables|Default|SetEmissive (+ (* _changed_ds 5e+01) (Variables|Default|GetEmissive))))
      (Rendering|Material|SetScalarParameterValue (Variables|Default|GetDyna%20Mat) "Emissive" _output_get_3 :!class /Script/Engine.MaterialInstanceDynamic))))

(fn ConstructionScript)

(fn ValueChange
  (params (Delta%20Second :type Float%20%28single-precision%29))
  (Utilities|FlowControl|Sequence
    (:then_0
      (if (<= (Variables|Default|GetEmissive) 0.0)
        (return Delta%20Second)))
    (:then_1
      (if (>= (Variables|Default|GetEmissive) 1e+02)
        (return (* Delta%20Second -1.0))))))