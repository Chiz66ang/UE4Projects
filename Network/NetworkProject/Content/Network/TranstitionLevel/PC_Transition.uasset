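; Player controller for the transition level that verifies the player's login and shows a session list UI.
; On BeginPlay, the local controller loads the player save and checks its ID and the GameInstance's PlayerID lookup of the slot name.
; On success it opens WG_Transition with UI-only input and a visible cursor.
; It then binds a GameInstance event that adds a named WG_SessionButton to the session list per call.
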(event Custom|Create%20widget
  ;[1 1 1] 위젯 생성/Add to Viewport
  (bind _returnvalue (UserInterface|CreateWidget "/Game/Network/TranstitionLevel/WG_Transition.WG_Transition_C" self))
  (bind _output_get (Variables|Default|SetTransitionWidget _returnvalue))
  (UserInterface|Viewport|AddtoViewport _output_get 0)
  (Input|SetInputModeUIOnly self 0 "DoNotLock")
  (Variables|Default|SetbShowMouseCursor true))

(event Custom|MakeSessionlist
  (params (SessionName :type String))
  (bind _returnvalue (UserInterface|CreateWidget "/Game/Network/TranstitionLevel/WG_SessionButton.WG_SessionButton_C" self))
  (Variables|/Game/Network/TranstitionLevel/WG_SessionButton.WG_SessionButton_C|SetSessionName _returnvalue SessionName)
  (Class|VerticalBox|AddChildtoVerticalBox (Variables|/Game/Network/TranstitionLevel/WG_Transition.WG_Transition_C|GetVerticalBox_SSlist (Variables|Default|GetTransitionWidget)) _returnvalue))

(event EventBeginPlay
  ;[1 1 1] 로그인 확인 후 위젯 생성
  (if (Pawn|IsLocalPlayerController)
    (bind _asgi_game_instance (Utilities|Casting|CastToGI_GameInstance (Game|GetGameInstance)))
    (bind _returnvalue (SaveGame|LoadGamefromSlot (Variables|/Game/Network/GI_GameInstance.GI_GameInstance_C|GetSG_SlotName _asgi_game_instance)))
    (bind _assg_player (Utilities|Casting|CastToSG_Player _returnvalue))
    (if (Utilities|Enum|NotEqual(Enum) (Variables|/Game/Network/SG_Player.SG_Player_C|GetPlayerID _assg_player) "")
      (bind _asgi_game_instance_2 (Utilities|Casting|CastToGI_GameInstance (Game|GetGameInstance)))
      (if (.ReturnValue (Utilities|Map|Find (Variables|/Game/Network/GI_GameInstance.GI_GameInstance_C|GetPlayerID _asgi_game_instance_2) (Variables|/Game/Network/GI_GameInstance.GI_GameInstance_C|GetSG_SlotName _asgi_game_instance)))
        (Development|PrintString "Success")
        (CallFunction|CreateWidget)
        (EventDispatchers|BindEventtoSSMakeButton _asgi_game_instance_2 (delegate Custom|MakeSessionlist))))))

(fn ConstructionScript)