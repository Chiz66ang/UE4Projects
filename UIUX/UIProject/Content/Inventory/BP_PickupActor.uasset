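; BP_PickupActor is a world pickup item that shows its icon and title and can be collected by the player character.
; BeginPlay fills the image and text widget components from PickupInfo and loops the image widget's item animation.
; Tick rotates the whole actor to face the player camera.
; Box overlap passes PickupInfo to ThirdPersonCharacter's ItemGet and destroys the actor only if it returns true.
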(event OnComponentBeginOverlap(BoxCollision)
  (params (OverlappedComponent :type Primitive%20Component%20Object%20Reference) (OtherActor :type Actor%20Object%20Reference) (OtherComp :type Primitive%20Component%20Object%20Reference) (OtherBodyIndex :type Integer) (bFromSweep :type Boolean) (SweepResult :type Hit%20Result%20Structure%20%28by%20ref%29))
  (bind _asthird_person_character (Utilities|Casting|CastToThirdPersonCharacter OtherActor))
  (bind _result (Default|ItemGet _asthird_person_character (Variables|Default|GetPickupInfo)))
  (if _result
    (Actor|DestroyActor)))

(event EventBeginPlay
  (bind _pickupinfo (Variables|Default|GetPickupInfo))
  (bind (_itemtitle _itemicon) (Utilities|Struct|BreakBP_ItemStruct _pickupinfo))
  (Utilities|FlowControl|Sequence
    (:then_0
      ;[1 1 1] 화면에 띄우기
      (if (Utilities|IsValid (.ItemIcon (Utilities|Struct|BreakBP_ItemStruct (Variables|Default|GetPickupInfo))))
        (bind _aswg_image_widget (Utilities|Casting|CastToWG_ImageWidget (UserInterface|GetUserWidgetObject (Variables|Default|GetImageWidget))))
        (Variables|/Game/Inventory/WG_ImageWidget.WG_ImageWidget_C|SetItemIcon _aswg_image_widget _itemicon)
        (bind _aswg_text_widget (Utilities|Casting|CastToWG_TextWidget (UserInterface|GetUserWidgetObject (Variables|Default|GetTextWidget))))
        (Variables|/Game/Inventory/WG_TextWidget.WG_TextWidget_C|SetTextString _aswg_text_widget _itemtitle)))
    (:then_1
      (bind _aswg_image_widget_2 (Utilities|Casting|CastToWG_ImageWidget (UserInterface|GetUserWidgetObject (Variables|Default|GetImageWidget)))
        (:then
          (UserInterface|Animation|PlayAnimation _aswg_image_widget_2 (Variables|/Game/Inventory/WG_ImageWidget.WG_ImageWidget_C|GetItemAnimation _aswg_image_widget_2) 0.0 0 "Forward" 1.0))
        (:CastFailed
          (Development|PrintString "CastFailed"))))))

(event Collision|EventActorBeginOverlap
  (params (OtherActor :type Actor%20Object%20Reference)))

(event EventTick
  (params (DeltaSeconds :type Float%20%28single-precision%29))
  (Transformation|SetActorRotation (Math|Rotator|FindLookatRotation (Transformation|GetActorLocation) (Camera|GetCameraLocation (Variables|/Script/Engine.PlayerController|GetPlayerCameraManager (Game|GetPlayerController 0))))))

(fn ConstructionScript)